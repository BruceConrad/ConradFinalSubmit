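; Penguin NPC that turns to face the player and shows its dialogue one line per interaction.
; At BeginPlay it caches FinalDialogue table rows matching its NPCID.
; Each interaction increments the line counter and displays the row matching ConversationID and line in a reused widget, closing and resetting unless exactly one matches.
; The player ending overlap also removes the widget, and the construction script tints the MysteriousAura effect.
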(event EventBeginPlay
  (|CallParentFunction)
  (bind _outrownames (DataTable|GetDataTableRowNames "/Game/Bruce_Blueprints/NPC_Blueprints/FinalDialogue.FinalDialogue"))
  (for _array_element _outrownames
    (bind _returnvalue (Utilities|GetDataTableRow "/Game/Bruce_Blueprints/NPC_Blueprints/FinalDialogue.FinalDialogue" _array_element)
      (:then
        (if (== (.NPC_ID (Utilities|Struct|BreakStruct_NPCStruct _returnvalue)) (Variables|Default|GetNPC_ID))
          (Utilities|Array|Add (Variables|Default|GetMyDialogue) _array_element))))))

(event Collision|EventActorBeginOverlap
  (params (OtherActor :type Actor%20Object%20Reference))
  (|CallParentFunction OtherActor) ; This node is disabled and will not be called.\nDrag off pins to build functionality.
)

(event EventTick
  (params (DeltaSeconds :type Float%20%28single-precision%29))
  (|CallParentFunction DeltaSeconds) ; This node is disabled and will not be called.\nDrag off pins to build functionality.
)

(event EventNPCInteraction
  (Math|Integer|IncrementInt (Variables|Default|GetLineCurrent)
    (:%20%20
      (CallFunction|CreateDialogue)
      (Transformation|SetActorRotation (Math|Rotator|MakeRotator 0.0 0.0 (.Yaw (Math|Rotator|BreakRotator (Math|Rotator|FindLookatRotation (Transformation|GetActorLocation) (Transformation|GetActorLocation (Game|GetPlayerCharacter 0))))))))))

(event Collision|EventActorEndOverlap
  (params (OtherActor :type Actor%20Object%20Reference))
  (Utilities|Casting|CastToFirstPersonCharacter OtherActor)
  (Widget|RemovefromParent (Variables|Default|GetDialogueWidget)))

(fn ConstructionScript
  (|CallParentFunction)
  (Effects|Components|ParticleSystem|SetColorParameter (Variables|Default|GetMysteriousAura) "FireColor" (Variables|Default|GetFireColor)))

(fn CreateDialogue
  (Utilities|IsValid (Variables|Default|GetDialogueWidget)
    (:Is%20Valid
      (bind _returnedline (CallFunction|GetDialogueLine))
      (Variables|/Game/Bruce_Blueprints/NPC_Blueprints/NPCWidgets/Dialogue_Widget.Dialogue_Widget_C|SetDialogueText (Variables|Default|GetDialogueWidget) _returnedline))
    (:Is%20Not%20Valid
      (bind _returnvalue (UserInterface|CreateWidget "/Game/Bruce_Blueprints/NPC_Blueprints/NPCWidgets/Dialogue_Widget.Dialogue_Widget_C" (Game|GetPlayerController 0)))
      (bind _output_get (Variables|Default|SetDialogueWidget _returnvalue))
      (UserInterface|Viewport|AddtoViewport _output_get 0)
      (bind _returnedline_2 (CallFunction|GetDialogueLine))
      (Variables|/Game/Bruce_Blueprints/NPC_Blueprints/NPCWidgets/Dialogue_Widget.Dialogue_Widget_C|SetDialogueText (Variables|Default|GetDialogueWidget) _returnedline_2))))

(fn GetDialogueLine
  (for _array_element (Variables|Default|GetMyDialogue)
    (bind _returnvalue (Utilities|GetDataTableRow "/Game/Bruce_Blueprints/NPC_Blueprints/FinalDialogue.FinalDialogue" _array_element)
      (:then
        (if (and (== (.Conversation_ID (Utilities|Struct|BreakStruct_NPCStruct _returnvalue)) (Variables|Default|GetConversation_ID)) (== (.Line_ID (Utilities|Struct|BreakStruct_NPCStruct _returnvalue)) (Variables|Default|GetLineCurrent)))
          (Utilities|Array|Add (LocalVariables|GetReturnedLines) (.Dialogue (Utilities|Struct|BreakStruct_NPCStruct _returnvalue)))))))
  (if (== (Utilities|Array|Length (LocalVariables|GetReturnedLines)) 1)
    (return (Utilities|Array|Get(acopy) (LocalVariables|GetReturnedLines)))
    (else
      (Widget|RemovefromParent (Variables|Default|GetDialogueWidget))
      (Variables|Default|SetDialogueWidget 0)
      (Variables|Default|SetLineCurrent 0))))